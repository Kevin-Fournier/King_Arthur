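; BP_Spawner is an enemy spawner that repeatedly spawns zombies at its own location once the GiJoe player's Time reaches a threshold.
; A one-time trigger from Tick starts a delayed, self-looping spawn chain whose interval is read from a timeline's Delay track.
; In parallel, timed delays unlock fast, then big enemies, which get a random chance to join each spawn where the spawner's CanSpawn flags allow.
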(event `self.ReceiveTick`
  (params (DeltaSeconds :type "Float (single-precision)"))
  (bind _asgi_joe (cast `/Game/Wanna_Be_Dead_Nation/GiJoe` (`GameplayStatics.GetPlayerCharacter` 0)))
  (if (>= (`/Game/Wanna_Be_Dead_Nation/GiJoe.Time` _asgi_joe) 1.0)
    (`/Engine/EditorBlueprintResources/StandardMacros.DoOnce` false
      (:`Completed`
        (`|ExecutionSequence`
          (:`then_0`
            (`KismetSystemLibrary.Delay` (`self.Startup Delay`))
            (`|SpawnActorFromClass` "/Game/Zombie_Enemies/Zombie_1/Zombie_1.Zombie_1_C" (`SceneComponent.K2_GetComponentToWorld` (`self.DefaultSceneRoot`)) "Undefined" "OverrideRootScale" null null :!label _label)
            (`|ExecutionSequence`
              (:`then_0`
                (`KismetSystemLibrary.Delay` (stale _delay))
                (goto _label))
              (:`then_1`
                (if (`self.BigEnemy`)
                  (if (`self.Can Spawn Big Enemy ?`)
                    (`KismetSystemLibrary.Delay` 0.8)
                    (if (<= (`KismetMathLibrary.RandomFloatInRange` 0.0 5.0) 1.0)
                      (`|SpawnActorFromClass` "/Game/Wanna_Be_Dead_Nation/Enemy1.Enemy1_C" (`SceneComponent.K2_GetComponentToWorld` (`self.DefaultSceneRoot`)) "Undefined" "OverrideRootScale" null null)))))
              (:`then_2`
                (if (`self.Fast Enemy`)
                  (if (`self.Can Spawn Fast Enemy ?`)
                    (`KismetSystemLibrary.Delay` 0.5)
                    (if (<= (`KismetMathLibrary.RandomFloatInRange` 0.0 5.0) 1.0)
                      (`|SpawnActorFromClass` "/Game/Wanna_Be_Dead_Nation/Enemy2.Enemy2_C" (`SceneComponent.K2_GetComponentToWorld` (`self.DefaultSceneRoot`)) "Undefined" "OverrideRootScale" null null)))))))
          (:`then_1`
            (bind (_direction _delay) (`Timeline|Timeline_0`)))
          (:`then_2`
            (`KismetSystemLibrary.Delay` 20.0)
            (set `self.Fast Enemy` true)
            (`KismetSystemLibrary.Delay` 20.0)
            (set `self.BigEnemy` true)))))))

(fn `UserConstructionScript`)