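; BP_Barrel is an explosive barrel that catches fire when shot and then explodes.
; Bullets overlapping the capsule are destroyed and counted; the first hit ignites the fire effect and starts a delayed detonation, which a third hit triggers immediately.
; A shared DoOnce guards the explosion, which removes the mesh, swaps fire for blast effect, briefly sets the sphere to overlap everything, then destroys the actor.
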(event `Impact`
  (if (>= (`self.Impact Numbers`) 1.0)
    (`ActorComponent.Activate` (`self.P_Fire`) true)
    (`|ExecutionSequence`
      (:`then_0`
        (`KismetSystemLibrary.Delay` 6.0)
        (`/Engine/EditorBlueprintResources/StandardMacros.DoOnce` false :!label _label
          (:`Completed`
            (`PrimitiveComponent.SetCollisionProfileName` (`self.Sphere`) "OverlapAll" true)
            (`ActorComponent.K2_DestroyComponent` (`self.SM_Barrel`))
            (`ActorComponent.Activate` (`self.P_Explosion`) true)
            (`SceneComponent.SetVisibility` (`self.P_Fire`) false false)
            (`KismetSystemLibrary.Delay` 0.1)
            (`ActorComponent.K2_DestroyComponent` (`self.Sphere`))
            (`KismetSystemLibrary.Delay` 0.9)
            (`self.K2_DestroyActor`))))
      (:`then_1`
        (if (>= (`self.Impact Numbers`) 3.0)
          (goto _label))))))

(event `self.ReceiveBeginPlay`
  (`/Engine/EditorBlueprintResources/StandardMacros.IsValid` self))

(event `self.Capsule.OnComponentBeginOverlap`
  (params (OverlappedComponent :type "PrimitiveComponent Object Reference") (OtherActor :type "Actor Object Reference") (OtherComp :type "PrimitiveComponent Object Reference") (OtherBodyIndex :type Integer) (bFromSweep :type Boolean) (SweepResult :type "HitResult Structure (by ref)"))
  (bind _asbp_bullet (cast `/Game/Wanna_Be_Toy_Story/BP_Bullet` OtherActor))
  (`self.K2_DestroyActor` _asbp_bullet)
  (set `self.Impact Numbers` (+ (`self.Impact Numbers`) 1.0))
  (`self.Impact`))

(fn `UserConstructionScript`)