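; BP_Spawner1 is an enemy spawner that continuously creates Zombie_1 actors at its root transform.
; On BeginPlay, once the player character casts to GiJoe, a Sequence starts a looping spawn-and-Delay cycle and plays a timeline with no visible outputs.
; A third branch uses staggered delays to raise FastEnemy, then BigEnemy, flags that this graph sets but never reads.
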(event `self.ReceiveBeginPlay`
  (cast `/Game/Wanna_Be_Toy_Story/GiJoe` (`GameplayStatics.GetPlayerCharacter` 0))
  (`/Engine/EditorBlueprintResources/StandardMacros.DoOnce` false
    (:`Completed`
      (`|ExecutionSequence`
        (:`then_0`
          (`|SpawnActorFromClass` "/Game/Zombie_Enemies/Zombie_1/Zombie_1.Zombie_1_C" (`SceneComponent.K2_GetComponentToWorld` (`self.DefaultSceneRoot`)) "Undefined" "OverrideRootScale" null null :!label _label)
          (`KismetSystemLibrary.Delay` 2.0)
          (goto _label))
        (:`then_1`
          (`Timeline|Timeline_0`))
        (:`then_2`
          (`KismetSystemLibrary.Delay` 20.0)
          (set `self.Fast Enemy` true)
          (`KismetSystemLibrary.Delay` 20.0)
          (set `self.BigEnemy` true))))))

(fn `UserConstructionScript`)