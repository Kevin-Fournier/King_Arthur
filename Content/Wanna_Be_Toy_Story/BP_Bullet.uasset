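; Projectile bullet that damages Zombie_1, Enemy1 and Enemy2 and supports the player's slow-motion state.
; Tick polls GiJoe's SlowDown flag, using two alternating DoOnce gates to switch between slowed and full speed while stopping or playing a timeline.
; Timeline updates feed a delayed self-destruct, and the bullet also destroys itself when it stops moving.
; One sphere overlap subtracts enemy Health and destroys the bullet; a second sphere destroys it on any overlap.
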(event `self.ReceiveBeginPlay`
  (`/Engine/EditorBlueprintResources/StandardMacros.IsValid` self
    (:`Is Valid`
      (bind _asgi_joe (cast `/Game/Wanna_Be_Toy_Story/GiJoe` (`GameplayStatics.GetPlayerCharacter` 0)))
      (set `self.As Gi Joe` _asgi_joe))))

(event `self.ReceiveTick`
  (params (DeltaSeconds :type "Float (single-precision)"))
  (bind _projectilemovement (`self.ProjectileMovement`))
  (if (<= (`KismetMathLibrary.VSize` (`MovementComponent.Velocity` (`self.ProjectileMovement`))) 0.0)
    (`self.K2_DestroyActor`)
    (elif (`/Game/Wanna_Be_Toy_Story/GiJoe.Slow Down` (`self.As Gi Joe`))
      (`/Engine/EditorBlueprintResources/StandardMacros.DoOnce` false :!label _label
        (:`Completed`
          (set `ProjectileMovementComponent.MaxSpeed` 100.0 _projectilemovement)
          (`|ExecutionSequence`
            (:`then_0`
              (`Timeline|Timeline_0` :!via `Stop` :!label _label_2
                (:`Update`
                  (`KismetSystemLibrary.Delay` 3.0)
                  (`self.K2_DestroyActor`))))
            (:`then_1`
              (goto _label_3 :!via `Reset`)))))
      (else
        (`/Engine/EditorBlueprintResources/StandardMacros.DoOnce` false :!label _label_3
          (:`Completed`
            (set `ProjectileMovementComponent.MaxSpeed` 2000.0 _projectilemovement)
            (`ProjectileMovementComponent.SetVelocityInLocalSpace` _projectilemovement (2000.0 0.0 0.0))
            (`|ExecutionSequence`
              (:`then_0`
                (goto _label_2))
              (:`then_1`
                (goto _label :!via `Reset`)))))))))

(event `self.Sphere.OnComponentBeginOverlap`
  (params (OverlappedComponent :type "PrimitiveComponent Object Reference") (OtherActor :type "Actor Object Reference") (OtherComp :type "PrimitiveComponent Object Reference") (OtherBodyIndex :type Integer) (bFromSweep :type Boolean) (SweepResult :type "HitResult Structure (by ref)"))
  (`|ExecutionSequence`
    (:`then_0`
      (bind _aszombie_1 (cast `/Game/Zombie_Enemies/Zombie_1/Zombie_1` OtherActor))
      (`/Engine/EditorBlueprintResources/StandardMacros.DoOnce` false
        (:`Completed`
          (set `/Game/Zombie_Enemies/Zombie_1/Zombie_1.Health` (- (`/Game/Zombie_Enemies/Zombie_1/Zombie_1.Health` _aszombie_1) 20.0) _aszombie_1))))
    (:`then_1`
      (bind _asenemy_1 (cast `/Game/Wanna_Be_Toy_Story/Enemy1` OtherActor))
      (`/Engine/EditorBlueprintResources/StandardMacros.DoOnce` false
        (:`Completed`
          (set `/Game/Wanna_Be_Toy_Story/Enemy1.Health` (- (`/Game/Wanna_Be_Toy_Story/Enemy1.Health` _asenemy_1) 20.0) _asenemy_1))))
    (:`then_2`
      (bind _asenemy_2 (cast `/Game/Wanna_Be_Toy_Story/Enemy2` OtherActor))
      (`/Engine/EditorBlueprintResources/StandardMacros.DoOnce` false
        (:`Completed`
          (set `/Game/Wanna_Be_Toy_Story/Enemy2.Health` (- (`/Game/Wanna_Be_Toy_Story/Enemy2.Health` _asenemy_2) 20.0) _asenemy_2)))))
  (`self.K2_DestroyActor`))

(event `self.Sphere1.OnComponentBeginOverlap`
  (params (OverlappedComponent :type "PrimitiveComponent Object Reference") (OtherActor :type "Actor Object Reference") (OtherComp :type "PrimitiveComponent Object Reference") (OtherBodyIndex :type Integer) (bFromSweep :type Boolean) (SweepResult :type "HitResult Structure (by ref)"))
  (`self.K2_DestroyActor`))

(fn `UserConstructionScript`)