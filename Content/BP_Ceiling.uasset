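; BP_Ceiling is a ceiling actor that disappears while the GiJoe character is beneath or inside it.
; Shortly after BeginPlay, it switches its Box to the Trigger collision profile with overlaps updated.
; Box overlap begin and end events, filtered by a cast to GiJoe, hide and restore the StaticMesh's visibility.
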(event `self.ReceiveBeginPlay`
  (`KismetSystemLibrary.Delay` 0.05)
  (`PrimitiveComponent.SetCollisionProfileName` (`self.Box`) "Trigger" true))

(event `self.Box.OnComponentBeginOverlap`
  (params (OverlappedComponent :type "PrimitiveComponent Object Reference") (OtherActor :type "Actor Object Reference") (OtherComp :type "PrimitiveComponent Object Reference") (OtherBodyIndex :type Integer) (bFromSweep :type Boolean) (SweepResult :type "HitResult Structure (by ref)"))
  (cast `/Game/Wanna_Be_Toy_Story/GiJoe` OtherActor)
  (`SceneComponent.SetVisibility` (`self.StaticMesh`) false false))

(event `self.Box.OnComponentEndOverlap`
  (params (OverlappedComponent :type "PrimitiveComponent Object Reference") (OtherActor :type "Actor Object Reference") (OtherComp :type "PrimitiveComponent Object Reference") (OtherBodyIndex :type Integer))
  (cast `/Game/Wanna_Be_Toy_Story/GiJoe` OtherActor)
  (`SceneComponent.SetVisibility` (`self.StaticMesh`) true false))

(fn `UserConstructionScript`)